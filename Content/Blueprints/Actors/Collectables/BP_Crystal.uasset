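; BP_Crystal is a collectable crystal that flies into the player when they overlap it, then destroys itself.
; On overlap with the player it stores its starting location, scale and light intensity, then plays CollectionTimeline.
; Separate timeline tracks drive lerps toward the player's current position, down to zero scale and to zero point light intensity.
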(event `self.ReceiveActorBeginOverlap`
  (params (OtherActor :type "Actor Object Reference"))
  (`/Game/Blueprints/Libraries/CC_MacroLibrary.IsPlayer` OtherActor
    (:`IsPlayer`
      (`self.StoreStartingValues`)
      (bind (_direction _collection_progress _scale_track _light_track) (`Timeline|CollectionTimeline`)
        (:`Update`
          (`self.MoveToPlayer` _collection_progress)
          (`self.ScaleCrystal` _scale_track)
          (`self.Adjust Light` _light_track))
        (:`Finished`
          (`self.K2_DestroyActor`))))))

(fn `Adjust Light`
  (params (Alpha :type "Float (double-precision)"))
  (`LightComponent.SetIntensity` (`self.PointLight`) (`KismetMathLibrary.Lerp` (`self.Starting Intensity`) 0.0 Alpha)))

(fn `MoveToPlayer`
  (params (Alpha :type "Float (single-precision)"))
  (`self.K2_SetActorLocation` (`KismetMathLibrary.VLerp` (`self.StartLocation`) (`self.K2_GetActorLocation` (`GameplayStatics.GetPlayerPawn` 0)) Alpha)))

(fn `ScaleCrystal`
  (params (Alpha :type "Float (single-precision)"))
  (`self.SetActorScale3D` (`KismetMathLibrary.VLerp` (`self.Start Scale`) (0.0 0.0 0.0) Alpha)))

(fn `StoreStartingValues`
  (set `self.StartLocation` (`self.K2_GetActorLocation`))
  (set `self.Start Scale` (`self.GetActorScale3D`))
  (set `self.Starting Intensity` (`LightComponentBase.Intensity` (`self.PointLight`))))

(fn `UserConstructionScript`)