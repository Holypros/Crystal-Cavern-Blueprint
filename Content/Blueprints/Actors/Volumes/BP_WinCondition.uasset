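; Win-condition volume that completes the level when the player overlaps it and no BP_Crystal actors remain in the world.
; Crystals are counted with GetAllActorsOfClass on each player overlap; if any remain, it prints how many.
; On completion it looks up the current level in the LevelNames array and opens the next one, or prints congratulations and quits the game after the last.
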(event `self.ReceiveActorBeginOverlap`
  (params (OtherActor :type "Actor Object Reference"))
  (bind (_result _length) (`self.AnyCrystalsRemaining`))
  (`/Game/Blueprints/Libraries/CC_MacroLibrary.IsPlayer` OtherActor
    (:`IsPlayer`
      (if _result
        (`KismetSystemLibrary.PrintString` (`KismetStringLibrary.Concat_StrStr` "There's still " (`KismetStringLibrary.Conv_IntToString` _length) " crystals remaining"))
        (else
          (`self.CompleteLevel`))))))

(fn `AnyCrystalsRemaining`
  (returns (Result :type Boolean) (Length :type Integer))
  (bind _outactors (`GameplayStatics.GetAllActorsOfClass` "/Game/Blueprints/Actors/Collectables/BP_Crystal.BP_Crystal_C"))
  (bind _returnvalue (`KismetArrayLibrary.Array_Length` _outactors))
  (return (> _returnvalue 0) _returnvalue))

(fn `CompleteLevel`
  (if (`self.Is Final Level`)
    (`KismetSystemLibrary.PrintString` "Congrats. You have completed all Levels")
    (`KismetSystemLibrary.QuitGame` null "Quit")
    (else
      (`self.LoadNextLevel`))))

(fn `Get Current Level Index`
  (returns (`Return Value` :type Integer))
  (bind _returnvalue (`GameplayStatics.GetCurrentLevelName` true))
  (return (`KismetArrayLibrary.Array_Find` (`self.LevelNames`) (`KismetStringLibrary.Conv_StringToName` _returnvalue))))

(fn `Is Final Level`
  (returns (`Return Value` :type Boolean))
  (return (== (`KismetArrayLibrary.Array_LastIndex` (`self.LevelNames`)) (`self.Get Current Level Index`))))

(fn `LoadNextLevel`
  (bind _result (`/Engine/EditorBlueprintResources/StandardMacros.IncrementInt` (`self.Get Current Level Index`))
    (:`  `
      (`GameplayStatics.OpenLevel` (`|GetArrayItem` (`self.LevelNames`) _result)))))

(fn `UserConstructionScript`)