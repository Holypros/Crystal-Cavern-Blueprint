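; Player pawn that rolls its physics mesh in response to movement input.
; Forward/back and right/left axes apply torque around Y and X respectively, scaled by a shared rotation multiplier.
; Torque is applied as an acceleration change, so the mesh's mass does not affect the response.
; On BeginPlay the player camera fades in.
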(event `self.ReceiveBeginPlay`
  (`PlayerCameraManager.StartCameraFade` :`self` (`GameplayStatics.GetPlayerCameraManager` 0) :`FromAlpha` 1.0 :`Duration` 3.0))

(event `InputAxis|Move Forwards/Backwards`
  (params (AxisValue :type "Float (single-precision)"))
  (`PrimitiveComponent.AddTorqueInRadians` (`self.mesh`) (`KismetMathLibrary.MakeVector` 0.0 (* AxisValue (`self.Multiplication Rotation`))) "None" true))

(event `InputAxis|Move Right/Left`
  (params (AxisValue :type "Float (single-precision)"))
  (`PrimitiveComponent.AddTorqueInRadians` (`self.mesh`) (`KismetMathLibrary.MakeVector` (* AxisValue (`self.Multiplication Rotation`))) "None" true))

(fn `UserConstructionScript`)